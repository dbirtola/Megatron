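; Game mode Blueprint for a turn-based battle game structured in turns, rounds and combats.
; BeginPlay adds the battle HUD and a round-state debug widget to the viewport, then calls StartGame.
; Turn, round and combat start/end events are present as empty hooks, with comments describing when turns, rounds and combats begin.
; Tick only forwards to the parent, and the construction script is empty.
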(event `self.ReceiveBeginPlay`
  (bind _returnvalue (`|CreateWidget` "/Game/Widgets/WBP_BattleHUDWidget.WBP_BattleHUDWidget_C" (`GameplayStatics.GetPlayerController` 0)))
  (`UserWidget.AddToViewport` _returnvalue 0)
  (bind _returnvalue_2 (`|CreateWidget` "/Game/Framework/WB_DEBUG_RoundState.WB_DEBUG_RoundState_C"))
  (`UserWidget.AddToViewport` _returnvalue_2 0)
  (`self.StartGame`))

(event `self.ReceiveTick`
  (params (DeltaSeconds :type "Float (single-precision)"))
  (`parent.ReceiveTick` 0.0))

(event `self.OnTurnStart`
  (params (bIsPlayerTurn :type Boolean))
  ;[1 1 1] Called whenever a new turn starts or ends
  (if bIsPlayerTurn
    _))

(event `self.OnTurnEnd`
  (params (bWasPlayerTurn :type Boolean))
  ;[1 1 1] Called whenever a new turn starts or ends
  (if bWasPlayerTurn
    _))

(event `self.OnRoundStart`
  ;[1 1 1] A new round starts after players finish learning new abilities, and right before the player takes their next turn.
)

(event `self.OnRoundEnd`
  ;[1 1 1] A new round starts after players finish learning new abilities, and right before the player takes their next turn.
)

(event `self.OnCombatStart`
  ;[1 1 1] A new combat starts after all enemies have been defeated and the new enemies have been generated
)

(event `self.OnCombatEnd`
  ;[1 1 1] A new combat starts after all enemies have been defeated and the new enemies have been generated
)

(fn `UserConstructionScript`)