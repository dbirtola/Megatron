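; Slime actor Blueprint with a health component and a widget health bar, which deals itself a small hit one second after BeginPlay.
; On damage, it prints current health, computes the clamped new value and uses a timeline to lerp the health bar toward it.
; A second timeline then drives the damage bar directly from its track value, with a DoOnce blocking animation restarts until both finish.
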(event `self.ReceiveBeginPlay`
  (`KismetSystemLibrary.Delay` 1.0)
  (`HealthComponent.TakeDamage` (`self.HealthComponent`) (make `Damage` null 1)))

(event `self.HealthComponent.OnTakeDamage`
  (params (DamagedActor :type "Actor Object Reference") (DamageCauser :type "Actor Object Reference") (Damage :type "Damage Structure"))
  (bind _healthcomponent (`self.HealthComponent`))
  (bind _healthcomponent_2 (`self.HealthComponent`))
  (`KismetSystemLibrary.PrintString` (`KismetStringLibrary.Conv_IntToString` (`HealthComponent.CurrentHealth` (`self.HealthComponent`))))
  (set `self.tempHealth` (`KismetMathLibrary.Clamp` (- (`HealthComponent.CurrentHealth` _healthcomponent) (`.BaseDamage` (break `Damage` Damage))) 0 (`HealthComponent.MaxHealth` _healthcomponent)))
  (`/Engine/EditorBlueprintResources/StandardMacros.DoOnce` false :!label _label
    (:`Completed`
      (bind _aswbp_health_bar (cast `/Game/UI/Health_UI/WBP_HealthBar` (`WidgetComponent.GetUserWidgetObject` (`self.HealthWidget`))))
      (bind (_direction _newtrack_0) (`Timeline|Timeline_0`)
        (:`Update`
          (`ProgressBar.SetPercent` (`/Game/UI/Health_UI/WBP_HealthBar.HealthBar` _aswbp_health_bar) (`KismetMathLibrary.NormalizeToRange` (`KismetMathLibrary.Lerp` (`KismetMathLibrary.Conv_IntToDouble` (`HealthComponent.CurrentHealth` _healthcomponent_2)) (`KismetMathLibrary.Conv_IntToDouble` (`self.tempHealth`)) _newtrack_0) 0.0 (`KismetMathLibrary.Conv_IntToDouble` (`HealthComponent.MaxHealth` _healthcomponent_2)))))
        (:`Finished`
          (bind (_direction_2 _newtrack_0_2) (`Timeline|Timeline_1`)
            (:`Update`
              (`ProgressBar.SetPercent` (`/Game/UI/Health_UI/WBP_HealthBar.DamageBar` _aswbp_health_bar) _newtrack_0_2))
            (:`Finished`
              (goto _label :!via `Reset`))))))))

(fn `UserConstructionScript`)