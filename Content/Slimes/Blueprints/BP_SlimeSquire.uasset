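; BP_SlimeSquire is a slime Blueprint with a health bar and visual feedback for learning or forgetting abilities.
; Damage events from HealthComponent push max and current health into the WBP_HealthBar inside HealthWidget and print both values for debugging.
; Shortly after BeginPlay it damages itself slightly, which triggers that update.
; The learned and forgot ability events spawn explosion and forget particle effects at its location.
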(event `self.ReceiveBeginPlay`
  (`KismetSystemLibrary.Delay` 1.0)
  (`HealthComponent.TakeDamage` (`self.HealthComponent`) (make `Damage` null 1)))

(event `self.HealthComponent.OnTakeDamage`
  (params (DamagedActor :type "Actor Object Reference") (DamageCauser :type "Actor Object Reference") (Damage :type "Damage Structure"))
  (bind _healthcomponent (`self.HealthComponent`))
  (bind _currenthealth (`HealthComponent.CurrentHealth` _healthcomponent))
  (bind _aswbp_health_bar (cast `/Game/UI/Health_UI/WBP_HealthBar` (`WidgetComponent.GetWidget` (`self.HealthWidget`)) :!pure true))
  (bind _output_get (set `/Game/UI/Health_UI/WBP_HealthBar.MaxHealth` (`HealthComponent.MaxHealth` _healthcomponent) _aswbp_health_bar))
  (`/Game/UI/Health_UI/WBP_HealthBar.SetHealth` _aswbp_health_bar _currenthealth)
  (`MegatronUtilitiesLibrary.PrintStringToChannel` (`KismetStringLibrary.Concat_StrStr` "Current Heatlh: " (`KismetStringLibrary.Conv_IntToString` _currenthealth)))
  (`MegatronUtilitiesLibrary.PrintStringToChannel` (`KismetStringLibrary.Concat_StrStr` "Max Heatlh: " (`KismetStringLibrary.Conv_IntToString` _output_get)) 7))

(event `self.OnLearnedAbility`
  (`GameplayStatics.SpawnEmitterAtLocation` "/Game/StarterContent/Particles/P_Explosion.P_Explosion" (`self.K2_GetActorLocation`)))

(event `self.OnForgotAbility`
  (`GameplayStatics.SpawnEmitterAtLocation` "/Game/VFX/Combat_FX/Forget/P_Forget.P_Forget" (`self.K2_GetActorLocation`)))

(fn `UserConstructionScript`)